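; Master Chief player character Blueprint that creates the player HUD and manages Halo-style shield and health, both stored on that widget.
; Damage drains the shield before health and updates the bars; shield hits restart a recharge delay.
; Tick counts the delay down, then refills the shield by a fixed step each frame.
; RestoreHealth refills health, while death swaps all widgets for the main menu, pauses the game and shows the cursor.
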(event `self.ReceiveBeginPlay`
  (bind _returnvalue (`|CreateWidget` "/Game/UI/PlayerUI/PlayerUI_bp.PlayerUI_bp_C" (`GameplayStatics.GetPlayerControllerFromID` (`GameplayStatics.GetPlayerControllerID` null))))
  (bind _output_get (set `self.PlayerUI` _returnvalue))
  (`PlayerWidget_cpp.SetCharcaterWeapons` _output_get self)
  (`UserWidget.AddToViewport` _output_get 0)
  (`ProgressBar.SetPercent` (`/Game/UI/PlayerUI/PlayerUI_bp.HealthBar` (`self.PlayerUI`)) 100.0)
  (`ProgressBar.SetPercent` (`/Game/UI/PlayerUI/PlayerUI_bp.ShieldBar` (`self.PlayerUI`)) 100.0))

(event `Damge`
  (params (Damge :type "Float (double-precision)"))
  (bind _playerui (`self.PlayerUI`))
  (bind _playerui_2 (`self.PlayerUI`))
  (set `self.RechargeShield` true)
  (set `self.Damage` Damge)
  (if (> (`PlayerWidget_cpp.shield` (`self.PlayerUI`)) 0.0)
    (bind _output_get (set `PlayerWidget_cpp.shield` (- (`PlayerWidget_cpp.shield` (`self.PlayerUI`)) (`self.Damage`)) _playerui))
    (`ProgressBar.SetPercent` (`/Game/UI/PlayerUI/PlayerUI_bp.ShieldBar` _playerui) (/ _output_get (`PlayerWidget_cpp.maxShield` (`self.PlayerUI`))))
    (set `self.TimeToRecharge` 6.0)
    (else
      (bind _output_get_2 (set `PlayerWidget_cpp.health` (- (`PlayerWidget_cpp.health` (`self.PlayerUI`)) (`self.Damage`)) _playerui_2))
      (`ProgressBar.SetPercent` (`/Game/UI/PlayerUI/PlayerUI_bp.HealthBar` _playerui_2) (/ _output_get_2 (`PlayerWidget_cpp.maxHealth` (`self.PlayerUI`))))
      (if (<= (`PlayerWidget_cpp.health` (`self.PlayerUI`)) 0.0)
        (`self.Die`)
        (set `self.TimeToRecharge` 6.0)))))

(event `Die`
  (`WidgetLayoutLibrary.RemoveAllWidgets`)
  (bind _returnvalue (`|CreateWidget` "/Game/UI/MainMenu/MainMenu.MainMenu_C"))
  (`UserWidget.AddToViewport` _returnvalue 0)
  (`GameplayStatics.SetGamePaused` true)
  (set `PlayerController.bShowMouseCursor` true (`GameplayStatics.GetPlayerControllerFromID` 0)))

(event `self.ReceiveTick`
  (params (DeltaSeconds :type "Float (single-precision)"))
  (bind _playerui (`self.PlayerUI`))
  (if (`self.RechargeShield`)
    (bind _output_get (set `self.TimeToRecharge` (- (`self.TimeToRecharge`) (`GameplayStatics.GetWorldDeltaSeconds`))))
    (if (<= _output_get 0.0)
      (if (<= (`PlayerWidget_cpp.shield` (`self.PlayerUI`)) (`PlayerWidget_cpp.maxShield` (`self.PlayerUI`)))
        (bind _output_get_2 (set `PlayerWidget_cpp.shield` (+ (`PlayerWidget_cpp.shield` (`self.PlayerUI`)) 2.0) _playerui))
        (bind _returnvalue (/ _output_get_2 (`PlayerWidget_cpp.maxShield` (`self.PlayerUI`))))
        (`ProgressBar.SetPercent` (`/Game/UI/PlayerUI/PlayerUI_bp.ShieldBar` _playerui) _returnvalue)
        (if (>= _returnvalue 1.0)
          (set `self.RechargeShield` false)
          (set `self.TimeToRecharge` 6.0))))))

(event `Key|LeftMouseButton`
  (params (Key :type "Key Structure")))

(event `RestoreHealth`
  (bind _playerui (`self.PlayerUI`))
  (set `PlayerWidget_cpp.health` (`PlayerWidget_cpp.maxHealth` _playerui) _playerui)
  (`ProgressBar.SetPercent` (`/Game/UI/PlayerUI/PlayerUI_bp.HealthBar` (`self.PlayerUI`)) 1.0))

(fn `UserConstructionScript`)